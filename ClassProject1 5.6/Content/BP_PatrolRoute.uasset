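; BP_PatrolRoute is a patrol path actor that supplies world-space waypoints from the points of its PatrolRoute spline.
; GetPointLocation returns the location of the spline point at the current index.
; IncrementSplineIndex steps that index by Direction and flips Direction at either end for a ping-pong route, printing a debug string on each flip.
; The event graph and construction script are empty, leaving both functions to external callers.
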(event EventBeginPlay)

(event Collision|EventActorBeginOverlap
  (params (OtherActor :type Actor%20Object%20Reference)))

(event EventTick
  (params (DeltaSeconds :type Float%20%28single-precision%29)))

(fn ConstructionScript)

(fn GetPointLocation
  (return (Spline|GetLocationatSplinePoint (Variables|Default|GetPatrol%20Route) (Variables|Default|GetSplinePointIndex) "World")))

(fn IncrementSplineIndex
  (bind _output_get (Variables|Default|SetSplinePointIndex (+ (Variables|Default|GetSplinePointIndex) (Variables|Default|GetDirection))))
  (if (or (== _output_get (- (Spline|GetNumberOfSplinePoints (Variables|Default|GetPatrol%20Route)) 1)) (== _output_get 0))
    (Variables|Default|SetDirection (* (Variables|Default|GetDirection) -1))
    (Development|PrintString "Hello")))