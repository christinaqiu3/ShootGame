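; BPC_Inventory is an inventory Blueprint that lets its owner pick up BP_Item actors.
; PickUpItem gets the owner's look direction through GetLookDirectionMessage and sphere-traces WorldStatic objects from the owner's location out to PickUpRange.
; A hit BP_Item is added to HeldObjects and the resulting index is printed, with no change made to the item itself.
; The event graph and construction script are empty.
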(event EventBeginPlay)

(event Collision|EventActorBeginOverlap
  (params (OtherActor :type Actor%20Object%20Reference)))

(event EventTick
  (params (DeltaSeconds :type Float%20%28single-precision%29)))

(fn ConstructionScript)

(fn PickUpItem
  (bind _defaultsceneroot (Variables|Default|GetDefaultSceneRoot))
  (bind _returnvalue (Components|GetOwner _defaultsceneroot))
  (bind _returnvalue_2 (Transformation|GetActorLocation _returnvalue))
  (bind _look_direction (Class|BPICharacter|GetLookDirection(Message) _returnvalue))
  (bind _outhit (Collision|SphereTraceForObjects _returnvalue_2 (+ (* _look_direction (Variables|Default|GetPick%20Up%20Range)) _returnvalue_2) 3e+01 (Utilities|Array|MakeArray "ObjectTypeQuery1") false 0 "None"))
  (if true
    (bind _asbp_item (Utilities|Casting|CastToBP_Item (.HitActor (Collision|BreakHitResult _outhit))))
    (bind _returnvalue_3 (Utilities|Array|Add (Variables|Default|GetHeld%20Objects) _asbp_item))
    (Development|PrintString (Utilities|String|ToString(Integer) _returnvalue_3))))