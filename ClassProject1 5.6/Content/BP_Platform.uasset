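; BP_Platform is a color-switch platform that appears or disappears when Tab is pressed.
; It enables input from the first player's controller on BeginPlay, then flips its own ShowRed flag on each press and compares it to ColorIsRed.
; SetPlatformActive toggles mesh visibility and collision to match, with debug prints on each switch.
; Platform state is first applied on a Tab press, as neither BeginPlay nor the construction script sets it.
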(event EventBeginPlay
  (Input|EnableInput (Game|GetPlayerController (Variables|/Script/Engine.Pawn|GetPlayerState (Game|Player|GetPlayerPawn 0)))))

(event Collision|EventActorBeginOverlap
  (params (OtherActor :type Actor%20Object%20Reference)))

(event EventTick
  (params (DeltaSeconds :type Float%20%28single-precision%29)))

(event Input|KeyboardEvents|Tab
  (params (Key :type Key%20Structure :default "None"))
  (:Pressed
    (Development|PrintString "tab")
    (bind _output_get (Variables|Default|SetbShowRed (not (Variables|Default|GetbShowRed))))
    (if (== _output_get (Variables|Default|GetcolorIsRed))
      (CallFunction|SetPlatformActive true)
      (Development|PrintString "active")
      (else
        (CallFunction|SetPlatformActive false)
        (Development|PrintString "not active")))))

(fn ConstructionScript)

(fn SetPlatformActive
  (params (bActive :type Boolean))
  (Rendering|SetVisibility (Variables|Default|GetStaticMesh) bActive false)
  (if bActive
    (Collision|SetCollisionEnabled (Variables|Default|GetStaticMesh) "QueryAndPhysics")
    (else
      (Collision|SetCollisionEnabled (Variables|Default|GetStaticMesh) "NoCollision"))))