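; BP_EnemyBullet is an enemy projectile that damages the first-person player.
; On BeginPlay it launches its Sphere with a physics impulse along a Direction variable.
; Overlapping the player pawn calls Damage on that character's BPHealthComponent.
; Disconnected nodes for ignoring WorldStatic collision and for a delayed random red or blue material never run.
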(event EventBeginPlay
  (Physics|AddImpulse (Variables|Default|GetSphere) (* (Variables|Default|Getdirection) 3e+03) "None" false))

(event Collision|EventActorBeginOverlap
  (params (OtherActor :type Actor%20Object%20Reference))
  (if (== (Game|Player|GetPlayerPawn 0) OtherActor)
    (bind _asbp_first_person_character (Utilities|Casting|CastToBP_FirstPersonCharacter OtherActor))
    (Default|Damage (Variables|/Game/FirstPerson/Blueprints/BP_FirstPersonCharacter.BP_FirstPersonCharacter_C|GetBP_HealthComponent _asbp_first_person_character))))

(event EventTick
  (params (DeltaSeconds :type Float%20%28single-precision%29)))

(fn ConstructionScript)