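; BP_CollectableCoin is a coin pickup that the first-person character collects by overlapping it.
; On overlap it plays a sound at the character's location and increments that character's CollectedCoins count.
; Instead of being destroyed, the coin then jumps by a random horizontal offset from its current position, so it can be collected repeatedly.
; A debug "hit" print fires for any overlapping actor, before the character cast.
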(event EventBeginPlay)

(event Collision|EventActorBeginOverlap
  (params (OtherActor :type Actor%20Object%20Reference))
  (bind _returnvalue (Math|Random|RandomIntegerinRange -300 300))
  (Development|PrintString "hit")
  (bind _asbp_first_person_character (Utilities|Casting|CastToBP_FirstPersonCharacter OtherActor))
  (Audio|SpawnSoundatLocation "/Engine/EditorSounds/Notifications/CompileSuccess.CompileSuccess" (Transformation|GetActorLocation _asbp_first_person_character) "0, 0, 0" 1.0 1.0 0.0 0 0)
  (Variables|/Game/FirstPerson/Blueprints/BP_FirstPersonCharacter.BP_FirstPersonCharacter_C|SetcollectedCoins _asbp_first_person_character (+ (Variables|/Game/FirstPerson/Blueprints/BP_FirstPersonCharacter.BP_FirstPersonCharacter_C|GetcollectedCoins _asbp_first_person_character) 1))
  (Transformation|SetActorLocation (+ (Transformation|GetActorLocation) (Math|Vector|MakeVector (Math|Conversions|ToFloat(Integer) _returnvalue) (Math|Conversions|ToFloat(Integer) _returnvalue) 0.0)) false false))

(event EventTick
  (params (DeltaSeconds :type Float%20%28single-precision%29)))

(fn ConstructionScript)