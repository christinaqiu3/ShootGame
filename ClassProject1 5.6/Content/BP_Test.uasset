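; Test actor that turns on gravity for its Sphere and spawns a spinning rifle pickup.
; BeginPlay spawns a BP_Pickup_Rifle at the actor's location and stores it in NewVar.
; Tick rotates that pickup by a fixed one-degree step each frame, not scaled by delta time.
; Overlap and click events are empty, and a few leftover nodes are unused.
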(event MouseInput|EventActorOnClicked
  (params (ButtonPressed :type Key%20Structure :default "None")))

(event Collision|EventActorBeginOverlap
  (params (OtherActor :type Actor%20Object%20Reference)))

(event EventBeginPlay
  (bind _output_get (Variables|Default|SetEnable%20Gravity true))
  (Physics|SetEnableGravity (Variables|Default|GetSphere) _output_get)
  (bind _returnvalue (Game|SpawnActorfromClass "/Game/FirstPerson/Blueprints/BP_Pickup_Rifle.BP_Pickup_Rifle_C" (Math|Transform|MakeTransform (Transformation|GetActorLocation)) "Undefined" "MultiplyWithRoot" 0 0))
  (Variables|Default|SetNewVar _returnvalue))

(event EventTick
  (params (DeltaSeconds :type Float%20%28single-precision%29))
  (bind _newvar (Variables|Default|GetNewVar))
  (Transformation|SetActorRotation _newvar (Math|Rotator|CombineRotators (Transformation|GetActorRotation _newvar) "0.000000,0.000000,1.000000")))

(fn ConstructionScript)