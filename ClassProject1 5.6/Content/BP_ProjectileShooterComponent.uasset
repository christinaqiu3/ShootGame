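; Projectile shooter component that fires BP_Projectile from the player pawn along a supplied camera's forward vector, limited by a charge count.
; Shoot spawns the projectile, sound and fire effect at a camera-relative offset, spends a charge and prints the remainder, or plays an invalid-action sound and smoke when empty.
; Each shot sets a looping RechargeDuration timer, apparently driving RechargeCharge, which restores one charge up to MaxCharges.
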(event Custom|RechargeCharge
  (if (< (Variables|Default|GetCurrentCharges) (Variables|Default|GetMaxCharges))
    (Math|Integer|IncrementInt (Variables|Default|GetCurrentCharges))))

(event EventBeginPlay
  (Variables|Default|SetCurrentCharges (Variables|Default|GetMaxCharges)))

(event EventTick
  (params (DeltaSeconds :type Float%20%28single-precision%29)))

(fn Shoot
  (params (Cam :type Camera%20Component%20Object%20Reference))
  (bind _returnvalue (Game|Player|GetPlayerPawn 0))
  (bind _returnvalue_2 (Math|Vector|GetUpVector Cam))
  (bind _returnvalue_3 (Transformation|GetActorLocation _returnvalue))
  (bind _returnvalue_4 (Math|Vector|GetForwardVector Cam))
  (bind _returnvalue_5 (* _returnvalue_2 "50.000000,50.000000,50.000000"))
  (bind _returnvalue_6 (* _returnvalue_4 "10.000000,10.000000,10.000000"))
  (bind _returnvalue_7 (+ _returnvalue_3 _returnvalue_5 _returnvalue_6))
  (if (> (Variables|Default|GetCurrentCharges) 0)
    (Audio|PlaySoundatLocation "/Game/FPWeapon/Audio/FirstPersonTemplateWeaponFire02.FirstPersonTemplateWeaponFire02" _returnvalue_7 "0, 0, 0" 1.0 1.0 0.0 0 0 0 0)
    (Effects|SpawnEmitteratLocation "/Game/StarterContent/Particles/P_Fire.P_Fire" _returnvalue_7)
    (Game|SpawnActorfromClass "/Game/BP_Projectile.BP_Projectile_C" (Math|Transform|MakeTransform _returnvalue_7 (Math|Rotator|MakeRotfromX _returnvalue_4)) "Undefined" "MultiplyWithRoot" 0 _returnvalue_4 0)
    (Math|Integer|DecrementInt (Variables|Default|GetCurrentCharges)
      (:%20%20
        (Utilities|Time|SetTimerbyEvent (EventDispatchers|CreateEvent :!event Custom|RechargeCharge) (Variables|Default|GetRechargeDuration) true)
        (Development|PrintText (Utilities|Text|ToText(Integer) (Variables|Default|GetCurrentCharges)))))
    (else
      (Audio|PlaySoundatLocation "/Engine/VREditor/Sounds/UI/Invalid_Action.Invalid_Action" _returnvalue_7 "0, 0, 0" 1.0 1.0 0.0 0 0 0 0)
      (Effects|SpawnEmitteratLocation "/Game/StarterContent/Particles/P_Smoke.P_Smoke" _returnvalue_7))))