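; BP_Target is a target actor that jumps to a new random spot when play begins and each time it is hit.
; BeginPlay and the Hit event both call TeleportRandomLocation, which sets the actor's location without sweeping.
; The new position is a random X and Y offset from a Center point within the SpawnRange bounds, at a fixed SpawnPosZ height.
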(event EventBeginPlay
  (CallFunction|TeleportRandomLocation))

(event Collision|EventActorBeginOverlap
  (params (OtherActor :type Actor%20Object%20Reference)))

(event EventTick
  (params (DeltaSeconds :type Float%20%28single-precision%29)))

(event Collision|EventHit
  (params (MyComp :type Primitive%20Component%20Object%20Reference) (Other :type Actor%20Object%20Reference) (OtherComp :type Primitive%20Component%20Object%20Reference) (bSelfMoved :type Boolean) (HitLocation :type Vector :default "0, 0, 0") (HitNormal :type Vector :default "0, 0, 0") (NormalImpulse :type Vector :default "0, 0, 0") (Hit :type Hit%20Result%20Structure%20%28by%20ref%29))
  (CallFunction|TeleportRandomLocation))

(fn ConstructionScript)

(fn TeleportRandomLocation
  (bind _spawnrange_x (Variables|Default|GetSpawnRange_X))
  (bind _spawnrange_y (Variables|Default|GetSpawnRange_Y))
  (bind _center (Variables|Default|GetCenter))
  (bind (_x _y) (Math|Vector|BreakVector _center))
  (Transformation|SetActorLocation (Math|Vector|MakeVector (+ _x (Math|Random|RandomFloatinRange (* _spawnrange_x -1.0) _spawnrange_x)) (+ _y (Math|Random|RandomFloatinRange (* _spawnrange_y -1.0) _spawnrange_y)) (Variables|Default|GetSpawnPos_Z)) false false))