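; BP_Spawner is a one-shot trigger that spawns a batch of BP_Target actors when a BP_FirstPersonCharacter enters its TriggerBox.
; A HasSpawned flag blocks repeat triggering, and a loop creates SpawnCount targets at the spawner's location.
; Each target receives SpawnRadius as its X and Y spawn range and the spawner's location as its center, so any spreading is left to BP_Target.
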(event OnComponentBeginOverlap(TriggerBox)
  (params (OverlappedComponent :type Primitive%20Component%20Object%20Reference) (OtherActor :type Actor%20Object%20Reference) (OtherComp :type Primitive%20Component%20Object%20Reference) (OtherBodyIndex :type Integer) (bFromSweep :type Boolean) (SweepResult :type Hit%20Result%20Structure%20%28by%20ref%29))
  (bind _returnvalue (Transformation|GetActorLocation))
  (bind _spawnradius (Variables|Default|GetSpawnRadius))
  (Utilities|Casting|CastToBP_FirstPersonCharacter OtherActor)
  (if (not (Variables|Default|GethasSpawned))
    (Variables|Default|SethasSpawned true)
    (for _index (range 0 (- (Variables|Default|GetSpawnCount) 1))
      (Game|SpawnActorfromClass "/Game/BP_Target.BP_Target_C" (Math|Conversions|ToTransform(Vector) _returnvalue) "Undefined" "MultiplyWithRoot" 0 _spawnradius _spawnradius _returnvalue 0))))

(event EventBeginPlay)

(event Collision|EventActorBeginOverlap
  (params (OtherActor :type Actor%20Object%20Reference)))

(event EventTick
  (params (DeltaSeconds :type Float%20%28single-precision%29)))

(fn ConstructionScript)