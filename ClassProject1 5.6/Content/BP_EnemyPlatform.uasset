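; BP_EnemyPlatform is a red-or-not colored platform that switches between solid and absent.
; Each SetPlatformActive call flips its ShowRed flag and marks the platform active when that matches its ColorIsRed setting.
; The active state drives the static mesh's visibility and collision, so an inactive platform is hidden and has no collision.
; The event graph and construction script are empty, and the file does not show what triggers the toggle.
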(event EventBeginPlay)

(event Collision|EventActorBeginOverlap
  (params (OtherActor :type Actor%20Object%20Reference)))

(event EventTick
  (params (DeltaSeconds :type Float%20%28single-precision%29)))

(fn ConstructionScript)

(fn SetPlatformActive
  (bind _output_get (Variables|Default|SetbShowRed (not (Variables|Default|GetbShowRed))))
  (if (== _output_get (Variables|Default|GetcolorIsRed))
    (Variables|Default|SetisActive true)
    (else
      (Variables|Default|SetisActive false)))
  (Rendering|SetVisibility (Variables|Default|GetStaticMesh) (Variables|Default|GetisActive) false)
  (if (Variables|Default|GetisActive)
    (Collision|SetCollisionEnabled (Variables|Default|GetStaticMesh) "QueryAndPhysics")
    (else
      (Collision|SetCollisionEnabled (Variables|Default|GetStaticMesh) "NoCollision"))))