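; Health component that tracks hit points and triggers the first-person player's death.
; CurrentHealth starts at MaxHealth, and each Damage call plays a test sine ping, lowers health by one and prints it.
; A call made with health already at zero or below stops the new sound and calls OnDeath on player pawn 0, whichever actor owns the component.
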(event EventBeginPlay
  (Variables|Default|SetCurrentHealth (Variables|Default|GetMaxHealth)))

(event EventTick
  (params (DeltaSeconds :type Float%20%28single-precision%29)))

(fn Damage
  (bind _returnvalue (Audio|SpawnSound2D "/Engine/EngineSounds/1kSineTonePing.1kSineTonePing" 1.0 1.0 0.0 0))
  (if (> (Variables|Default|GetCurrentHealth) 0.0)
    (bind _result (Math|Float|DecrementFloat (Variables|Default|GetCurrentHealth))
      (:%20%20
        (Development|PrintString (Utilities|String|ToString(Float) _result))))
    (else
      (Audio|Components|Audio|Stop _returnvalue)
      (bind _asbp_first_person_character (Utilities|Casting|CastToBP_FirstPersonCharacter (Game|Player|GetPlayerPawn 0)))
      (Default|OnDeath _asbp_first_person_character)
      (Development|PrintString "Player is dead"))))