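; Damage volume that periodically hurts players and enemies standing inside its TriggerBox.
; Overlap events add or remove each character's BPHealthComponent in a player or enemy array and set matching overlap flags.
; Tick runs through a one-second Delay, then calls Damage on every stored player component, or on enemy components only when the player flag is off.
; Any exit clears the player flag, and non-player exits also clear the enemy flag, even with others still inside.
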(event OnComponentBeginOverlap(TriggerBox)
  (params (OverlappedComponent :type Primitive%20Component%20Object%20Reference) (OtherActor :type Actor%20Object%20Reference) (OtherComp :type Primitive%20Component%20Object%20Reference) (OtherBodyIndex :type Integer) (bFromSweep :type Boolean) (SweepResult :type Hit%20Result%20Structure%20%28by%20ref%29))
  (bind _asbp_first_person_character (Utilities|Casting|CastToBP_FirstPersonCharacter OtherActor)
    (:then
      (Utilities|Array|Add (Variables|Default|GetBP%20Health%20Component) (Variables|/Game/FirstPerson/Blueprints/BP_FirstPersonCharacter.BP_FirstPersonCharacter_C|GetBP_HealthComponent _asbp_first_person_character))
      (Development|PrintString "player damage")
      (Variables|Default|SetplayerOverlapping true))
    (:CastFailed
      (bind _asbp_enemy_base (Utilities|Casting|CastToBP_Enemy_Base OtherActor))
      (Utilities|Array|Add (Variables|Default|GetBP%20Enemy%20Component) (Variables|/Game/FirstPerson/Blueprints/BP_FirstPersonCharacter.BP_FirstPersonCharacter_C|GetBP_HealthComponent _asbp_enemy_base))
      (Development|PrintString "enemy damage")
      (Variables|Default|SetenemyOverlapping true))))

(event OnComponentEndOverlap(TriggerBox)
  (params (OverlappedComponent :type Primitive%20Component%20Object%20Reference) (OtherActor :type Actor%20Object%20Reference) (OtherComp :type Primitive%20Component%20Object%20Reference) (OtherBodyIndex :type Integer))
  (Variables|Default|SetplayerOverlapping false)
  (bind _asbp_first_person_character (Utilities|Casting|CastToBP_FirstPersonCharacter OtherActor)
    (:then
      (Utilities|Array|RemoveItem (Variables|Default|GetBP%20Health%20Component) (Variables|/Game/FirstPerson/Blueprints/BP_FirstPersonCharacter.BP_FirstPersonCharacter_C|GetBP_HealthComponent _asbp_first_person_character)))
    (:CastFailed
      (Variables|Default|SetenemyOverlapping false)
      (bind _asbp_enemy_base (Utilities|Casting|CastToBP_Enemy_Base OtherActor))
      (Utilities|Array|RemoveItem (Variables|Default|GetBP%20Enemy%20Component) (Variables|/Game/FirstPerson/Blueprints/BP_FirstPersonCharacter.BP_FirstPersonCharacter_C|GetBP_HealthComponent _asbp_enemy_base)))))

(event EventBeginPlay)

(event Collision|EventActorBeginOverlap
  (params (OtherActor :type Actor%20Object%20Reference)))

(event EventTick
  (params (DeltaSeconds :type Float%20%28single-precision%29))
  (Utilities|FlowControl|Delay 1.0)
  (if (Variables|Default|GetplayerOverlapping)
    (for _array_element (Variables|Default|GetBP%20Health%20Component)
      (Default|Damage _array_element)
      (Development|PrintString "DAMAGING PLAYER"))
    (elif (Variables|Default|GetenemyOverlapping)
      (for _array_element_2 (Variables|Default|GetBP%20Enemy%20Component)
        (Default|Damage _array_element_2)
        (Development|PrintString "DAMAGING ENEMY")))))

(fn ConstructionScript)